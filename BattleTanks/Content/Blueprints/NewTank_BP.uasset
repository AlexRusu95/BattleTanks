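; Player-controllable tank Blueprint that handles driving, camera aiming, firing and a widget health bar.
; BeginPlay hands barrel, turret and tracks to the TankAiming and TankMovement components, then links the health bar to itself.
; Input drives track movement and firing through those components, while separate azimuth and spring arm rotations orbit the camera.
; Extra inputs spin the actor directly or attempt to right a flipped tank with force and rotation.
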(event `self.ReceiveBeginPlay`
  (`TankAimingComponent.Initialise` (`self.TankAiming`) (`self.TankBarrel`) (`self.TankTurret`))
  (`TankMovementComponent.Initialise` (`self.TankMovement`) (`self.TankTrackLeft`) (`self.TankTrackRight`))
  (`self.Initialise HealthBar` self))

(event `InputAxis|AimAzimuth`
  (params (AxisValue :type "Float (single-precision)"))
  ;[1 1 1] Camera / Aim
  (`SceneComponent.K2_AddLocalRotation` (`self.AzimuthAxis`) (`KismetMathLibrary.MakeRotator` 0.0 0.0 (* AxisValue (`GameplayStatics.GetWorldDeltaSeconds`) 100.0)) false false))

(event `InputAxis|Forward`
  (params (AxisValue :type "Float (single-precision)"))
  ;[1 1 1] Movement Input Binding
  (`TankMovementComponent.IntendMoveForward` (`self.TankMovement`) AxisValue))

(event `InputAxis|TurnRight`
  (params (AxisValue :type "Float (single-precision)"))
  ;[1 1 1] Movement Input Binding
  (`TankMovementComponent.IntendTurnRight` (`self.TankMovement`) AxisValue))

(event `InputAxis|AimElevate`
  (params (AxisValue :type "Float (single-precision)"))
  ;[1 1 1] Camera / Aim
  (`SceneComponent.K2_AddLocalRotation` (`self.SpringArm`) (`KismetMathLibrary.MakeRotator` 0.0 (* AxisValue (`GameplayStatics.GetWorldDeltaSeconds`) 100.0)) false false))

(event `InputAxis|SpinRotate`
  (params (AxisValue :type "Float (single-precision)"))
  ;[1 1 1] Movement Input Binding
  (`self.K2_AddActorLocalRotation` self (`KismetMathLibrary.MakeRotator` 0.0 0.0 (* AxisValue (`self.Rotation`) (`GameplayStatics.GetWorldDeltaSeconds`))) false false))

(event `InputAction|Fire`
  (params (Key :type "Key Structure"))
  ;[1 1 1] Camera / Aim
  (:`Pressed`
    (`TankAimingComponent.Fire` (`self.TankAiming`))))

(event `InputAction|Reset`
  (params (Key :type "Key Structure"))
  ;[1 1 1] Resets player rotation if upside down
  (:`Pressed`
    (`PrimitiveComponent.AddForceAtLocationLocal` (`self.Body`) (0.0 0.0 500.0) (`KismetMathLibrary.GetUpVector` (struct)) "None")
    (`self.K2_AddActorWorldRotation` self (`KismetMathLibrary.RLerp` (struct :`Roll` 1.0) (struct :`Roll` 180.0) (`self.Rotation`)) false false)))

(fn `Initialise HealthBar`
  (bind _ashealth_bar (cast `/Game/UI/HealthBar` (`WidgetComponent.GetUserWidgetObject` (`self.WidgetHealthBar`))))
  (set `/Game/UI/HealthBar.MyTank` self _ashealth_bar))

(fn `UserConstructionScript`)